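; BP_Item is an item that can be rotated between two orientations, with an icon and a two-axis size for each.
; Rotate toggles the IsRotated flag, which the other functions read.
; GetIconOrianted returns IconRotated or Icon based on that flag, and GetDimensions swaps X and Y when rotated, leaving the stored Dimensions untouched.
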(fn GetIconOrianted
  (return (select (Variables|Inventory|GetIsRotated) (Variables|Inventory|GetIconRotated) (Variables|Inventory|GetIcon))))

(fn Rotate
  (Variables|Inventory|SetIsRotated (not (Variables|Inventory|GetIsRotated))))

(fn GetDimensions
  (bind _dimensions (Variables|Inventory|GetDimensions))
  (if (Variables|Inventory|GetIsRotated)
    (return (Utilities|Struct|MakeIntPoint (.y _dimensions) (.x _dimensions)))
    (else
      (return (Variables|Inventory|GetDimensions)))))