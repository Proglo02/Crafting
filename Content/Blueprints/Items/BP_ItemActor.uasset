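; World pickup actor that represents an inventory item and can be collected by a player through interaction.
; The construction script sets the mesh from the ItemClass defaults, falling back to a chamfer cube.
; BeginPlay binds to BPInteractable and constructs an Item object from ItemClass if none is valid.
; Interacting passes the Item to the player's InventoryComponent and destroys the actor only if it is added.
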(event Custom|Interacted
  (params (PlayerRef :type BP%20First%20Person%20Character%20Object%20Reference))
  (bind _added (Default|TryAddItem (Variables|/Game/FPTemplate/FirstPerson/Blueprints/BP_FirstPersonCharacter.BP_FirstPersonCharacter_C|GetInventoryComponent PlayerRef) (Variables|Private|GetItem)))
  (if _added
    (Actor|DestroyActor)))

(event EventBeginPlay
  (EventDispatchers|BindEventtoInteracted (Variables|Default|GetBP_Interactable) (delegate Custom|Interacted))
  (Utilities|IsValid (Variables|Private|GetItem)
    (:Is%20Not%20Valid
      (bind _item (Private|CreateDefaultItem))
      (Variables|Private|SetItem _item))))

(fn ConstructionScript
  (bind _itemclass (Variables|Protected|GetItemClass)
    (:then
      (Utilities|IsValid (.ItemMesh (Utilities|GetClassDefaults _itemclass))
        (:Is%20Valid
          (Components|StaticMesh|SetStaticMesh (Variables|Default|GetStaticMesh) (.ItemMesh (Utilities|GetClassDefaults _itemclass))))
        (:Is%20Not%20Valid
          (Components|StaticMesh|SetStaticMesh (Variables|Default|GetStaticMesh) "/Game/Maps/LevelPrototyping/Meshes/SM_ChamferCube.SM_ChamferCube" :!label _label))))
    (:else
      (goto _label))))

(fn CreateDefaultItem
  (bind _itemclass (Variables|Protected|GetItemClass)
    (:then
      (bind _returnvalue (Game|ConstructObjectfromClass _itemclass))
      (return _returnvalue))
    (:else)))

(fn GetDefaultItem
  (return 0))