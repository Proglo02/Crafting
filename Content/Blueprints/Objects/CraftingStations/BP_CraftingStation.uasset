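; BP_CraftingStation is a world object that opens a crafting menu for the player when interacted with.
; On BeginPlay it caches the first-person character, binds to its BPInteractable component and creates a padded WB_CraftWidget fed by its BPInventoryComponent.
; Interacting passes that pre-built widget to the player's AddMenu, so the same widget instance is reused each time.
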(event Custom|Interacted
  (bind _playerref (Variables|Default|GetPlayerRef)
    (:then
      (Default|AddMenu _playerref (Variables|Default|GetCraftWidget)))
    (:else)))

(event EventBeginPlay
  (Utilities|FlowControl|Sequence
    (:then_0
      (bind _asbp_first_person_character (Utilities|Casting|CastToBP_FirstPersonCharacter (Game|Player|GetPlayerPawn 0)))
      (Variables|Default|SetPlayerRef _asbp_first_person_character))
    (:then_1
      (EventDispatchers|BindEventtoInteracted (Variables|Default|GetBP_Interactable) (delegate Custom|Interacted))
      (bind _returnvalue (UserInterface|CreateWidget "/Game/Blueprints/UI/Inventory/WB_CraftWidget.WB_CraftWidget_C" (Default|GetPlayerController (Variables|Default|GetPlayerRef)) (Variables|Default|GetBP_InventoryComponent) 5e+01))
      (bind _output_get (Variables|Default|SetCraftWidget _returnvalue))
      (Layout|BorderSlot|SetPadding _output_get (Utilities|Struct|MakeMargin 5e+01 0.0 0.0 0.0) :!class /Script/UMG.UserWidget))))

(fn ConstructionScript)